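; Gameplay ability for full-auto ranged fire, spawning projectiles at a set fire rate until input is released.
; It commits and builds one reduced-damage effect spec on activation, passed to every projectile.
; Each shot traces from the camera to correct muzzle aim for closer objects, clamps rotation using weapon handler data, and plays muzzle effects and sound.
; A delay loops the firing, while an input-release task created each shot ends the ability.
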(event `self.K2_ActivateAbility`
  (bind _returnvalue (`Actor.GetComponentByClass` (`self.GetAvatarActorFromActorInfo`) "/Game/Weapons/BComp_WeaponHandler.BComp_WeaponHandler_C"))
  (bind _returnvalue_2 (`Actor.GetComponentByClass` (`self.GetAvatarActorFromActorInfo`) "/Script/Engine.CameraComponent"))
  (bind (_returnvalue_roll _returnvalue_pitch _returnvalue_yaw) (`KismetMathLibrary.BreakRotator` (`Actor.K2_GetActorRotation` (`self.GetAvatarActorFromActorInfo`))))
  (bind _returnvalue_3 (`SceneComponent.K2_GetComponentLocation` _returnvalue_2))
  (bind _returnvalue_4 (`SceneComponent.GetSocketTransform` (`/Game/Weapons/WeaponBase/B_BaseWeaponInstance.WeaponMesh` (`/Game/Weapons/BComp_WeaponHandler.Weapon Ref` _returnvalue)) "Muzzle" "RTS_World"))
  (bind _location (.location _returnvalue_4))
  (bind _location_2 (.location _returnvalue_4))
  (`self.K2_CommitAbility`)
  (bind _gameplayeffectspechandle (`/Game/Libraries/FunctionLibrary.Make Gameplay Effect Damage` (`self.GetAvatarActorFromActorInfo`) 0.3))
  (set `self.ButtonDown` true)
  (if (`self.ButtonDown`) :!label _label
    ;[1 1 1] Line traces from camera to check if aim needs to get adjusted for closer objects
    (bind (_outhit _returnvalue_5) (`KismetSystemLibrary.LineTraceSingleForObjects` :`Start` _returnvalue_3 :`End` (+ _returnvalue_3 (* (`SceneComponent.GetForwardVector` _returnvalue_2) 3000.0)) :`ObjectTypes` (`|MakeArray` "ObjectTypeQuery1" "ObjectTypeQuery3" :!type "EObjectTypeQuery Enum") :`DrawTime` 1.5))
    (bind (_bblockinghit _binitialoverlap _time _distance _location_3 _impactpoint _normal _impactnormal _physmat _hitactor _hitcomponent _hitbonename _bonename _hititem _elementindex _faceindex _tracestart _traceend) (`GameplayStatics.BreakHitResult` _outhit))
    (`|SpawnActorFromClass` "/Game/Weapons/TestingStuff/BP_Projectile.BP_Projectile_C" (`KismetMathLibrary.MakeTransform` _location_2 (`/Game/Libraries/FunctionLibrary.ClampProjectileRotation` _returnvalue_yaw (.roll (`KismetMathLibrary.Conv_VectorToRotator` (`KismetMathLibrary.GetDirectionUnitVector` _location_2 (`KismetMathLibrary.SelectVector` _impactpoint _traceend _returnvalue_5)))) (.pitch (`KismetMathLibrary.Conv_VectorToRotator` (`KismetMathLibrary.GetDirectionUnitVector` _location_2 (`KismetMathLibrary.SelectVector` _impactpoint _traceend _returnvalue_5)))) (.yaw (`KismetMathLibrary.Conv_VectorToRotator` (`KismetMathLibrary.GetDirectionUnitVector` _location_2 (`KismetMathLibrary.SelectVector` _impactpoint _traceend _returnvalue_5)))) (`.RotationClamp_2_3932B28F4C5FA4F5218A4FBEDA5A4717` (break `/Game/GAS/AbilityInfo/RangedAbilityInfo` (`/Game/Weapons/BComp_WeaponHandler.Struct_RangedInfo` _returnvalue))))) "Undefined" "MultiplyWithRoot" (`self.GetAvatarActorFromActorInfo`) _gameplayeffectspechandle null)
    (`NiagaraFunctionLibrary.SpawnSystemAtLocation` "/Game/VFX/NS_MuzzleBurst.NS_MuzzleBurst" _location (.rotation _returnvalue_4))
    (`GameplayStatics.PlaySoundAtLocation` "/Game/SFX/SC_GunShot_01.SC_GunShot_01" _location (struct) 0.1 2.0 0.0 null null null null)
    (`AbilityTask_WaitInputRelease.WaitInputRelease` false
      (:`then`
        (`KismetSystemLibrary.Delay` (/ 1.0 (`self.FireRatePerSecond`)))
        (goto _label))
      (:`OnRelease`
        (set `self.ButtonDown` false)
        (`self.K2_EndAbility`)))
    (else
      (`self.K2_EndAbility`))))