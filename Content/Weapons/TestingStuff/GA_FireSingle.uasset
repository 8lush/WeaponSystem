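; GA_FireSingle is a Gameplay Ability that fires one projectile from the avatar's current weapon per activation.
; It commits, builds a GE_BasicDamage spec with SetByCaller damage, and passes it to a BP_Projectile spawned at the weapon's Muzzle socket.
; Projectile rotation comes from the character's base aim, clamped relative to actor yaw.
; Muzzle VFX and gunshot sound play at the socket, and the ability ends on input release.
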(event `self.K2_ActivateAbility`
  (bind _returnvalue (`AbilitySystemBlueprintLibrary.GetAbilitySystemComponent` (`self.GetAvatarActorFromActorInfo`)))
  (bind _returnvalue_2 (`SceneComponent.GetSocketTransform` (`/Game/Weapons/WeaponBase/B_BaseWeaponInstance.WeaponMesh` (`/Game/Weapons/BComp_WeaponHandler.Weapon Ref` (`Actor.GetComponentByClass` (`self.GetAvatarActorFromActorInfo`) "/Game/Weapons/BComp_WeaponHandler.BComp_WeaponHandler_C"))) "Muzzle" "RTS_World"))
  (bind _location (.location _returnvalue_2))
  (`self.K2_CommitAbility`)
  (bind _returnvalue_3 (`AbilitySystemBlueprintLibrary.AssignTagSetByCallerMagnitude` (`AbilitySystemComponent.MakeOutgoingSpec` _returnvalue "/Game/GAS/GameplayEffects/GE_BasicDamage.GE_BasicDamage_C" 0.0 (`AbilitySystemComponent.MakeEffectContext` _returnvalue)) (struct :`TagName` "Damage.SetByCaller") (`self.Damage`)))
  (bind _asbp_third_person_character (cast `/Game/ThirdPerson/CharacterBlueprints/BP_ThirdPersonCharacter` (`self.GetAvatarActorFromActorInfo`)))
  (bind (_returnvalue_roll _returnvalue_pitch _returnvalue_yaw) (`KismetMathLibrary.BreakRotator` (`Actor.K2_GetActorRotation` _asbp_third_person_character)))
  (bind (_returnvalue_roll_2 _returnvalue_pitch_2 _returnvalue_yaw_2) (`KismetMathLibrary.BreakRotator` (`Pawn.GetBaseAimRotation` _asbp_third_person_character)))
  (`|SpawnActorFromClass` "/Game/Weapons/TestingStuff/BP_Projectile.BP_Projectile_C" (`KismetMathLibrary.MakeTransform` (.location _returnvalue_2) (`/Game/Libraries/FunctionLibrary.ClampProjectileRotation` _returnvalue_yaw _returnvalue_roll_2 _returnvalue_pitch_2 _returnvalue_yaw_2 (`self.RotationClamp`))) "Undefined" "MultiplyWithRoot" (`self.GetAvatarActorFromActorInfo`) _returnvalue_3 null)
  (`NiagaraFunctionLibrary.SpawnSystemAtLocation` "/Game/VFX/NS_MuzzleBurst.NS_MuzzleBurst" _location (.rotation _returnvalue_2))
  (`GameplayStatics.PlaySoundAtLocation` "/Game/SFX/SC_GunShot_01.SC_GunShot_01" _location (struct) 0.4 1.5 0.0 null null null null)
  (`AbilityTask_WaitInputRelease.WaitInputRelease` false
    (:`OnRelease`
      (`self.K2_EndAbility`))))