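; Test punch attack gameplay ability that lunges the avatar a short distance forward and damages what it hits.
; After committing, it starts a root motion move and a sped-up punch montage together, then waits for one hit gameplay event.
; The event's target data receives a gameplay effect with SetByCaller damage, and hit actor names are printed for debugging.
; The ability ends when the montage finishes or is interrupted, or if commit fails.
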(event `self.K2_ActivateAbility`
  (bind _returnvalue (`self.GetAvatarActorFromActorInfo`))
  (bind _returnvalue_2 (`self.K2_CommitAbility`))
  (if _returnvalue_2
    (`AbilityTask_ApplyRootMotionMoveToForce.ApplyRootMotionMoveToForce` "None" (+ (* (`Actor.GetActorForwardVector` _returnvalue) 50.0) (`Actor.K2_GetActorLocation` _returnvalue)) 0.2 false "MOVE_None" false null "MaintainLastRootMotionVelocity"
      (:`then`
        (`AbilityTask_PlayMontageAndWait.CreatePlayMontageAndWaitProxy` "None" "/Game/Ninja_Starter/Animation/IPC/AM_TestPunch.AM_TestPunch" 2.5
          (:`then`
            (bind (_asynctaskproxy _payload) (`AbilityTask_WaitGameplayEvent.WaitGameplayEvent` (struct :`TagName` "Tests.Event.Hit") null true)
              (:`EventReceived`
                (bind _returnvalue_3 (`AbilitySystemBlueprintLibrary.AssignTagSetByCallerMagnitude` (`self.MakeOutgoingGameplayEffectSpec` (`self.GameplayEffect`)) (struct :`TagName` "Damage.SetByCaller") (`self.Damage`)))
                (bind (_eventtag _instigator _target _optionalobject _optionalobject2 _contexthandle _instigatortags _targettags _eventmagnitude _targetdata) (break `GameplayEventData` _payload))
                (`self.K2_ApplyGameplayEffectSpecToTarget` _returnvalue_3 _targetdata)
                (for _array_element (`AbilitySystemBlueprintLibrary.GetActorsFromTargetData` _targetdata)
                  (`KismetSystemLibrary.PrintString` (`KismetTextLibrary.Conv_TextToString` (`|FormatText` "Target hit: {Target Name}" (`KismetTextLibrary.Conv_StringToText` (`KismetSystemLibrary.GetDisplayName` _array_element)))) true true (struct :`R` 0.806952 :`G` 0.417885 :`A` 1.0) 2.0 "None")))))
          (:`OnCompleted`
            (`self.K2_EndAbility` :!label _label))
          (:`OnBlendOut`
            (goto _label))
          (:`OnInterrupted`
            (goto _label))
          (:`OnCancelled`
            (goto _label)))))
    (else
      (goto _label))))

(event `self.K2_OnEndAbility`
  (params (bWasCancelled :type Boolean))
  (`KismetSystemLibrary.PrintString` "Ability Ended" true true (struct :`G` 0.66 :`B` 1.0 :`A` 1.0) 2.0 "AbilityEnded"))