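; Gameplay ability that performs a multi-hit melee combo using attack chain data from the avatar's weapon handler component.
; Each step plays an attack montage, optionally with forward root motion force, and applies damage to targets from a hit gameplay event.
; A recovery montage follows, during which input advances the chain, requiring button release first unless auto-chain is set.
; Chain position, looping and input state decide when the ability ends.
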(event `self.K2_OnEndAbility`
  (params (bWasCancelled :type Boolean))
  (`KismetSystemLibrary.PrintString` "Ability Ended" true true (struct :`G` 0.66 :`B` 1.0 :`A` 1.0) 2.0 "AbilityEnded"))

(event `self.K2_ActivateAbility`
  (bind _returnvalue (`self.GetAvatarActorFromActorInfo`))
  (bind _currentattack (`self.CurrentAttack`))
  (bind (_usesforwardrootmotion _rootmotionduration _rootmotionforce _attackanimation _attackanimplayrate _attackdamagemultiplier _recoveryanimation _recoveryanimplayrate) (break `/Game/GAS/AbilityInfo/MeleeAbilityInfo_Attack` (`|GetArrayItem` (`self.Struct Melee Info Attacks`) _currentattack)))
  (bind _returnvalue_2 (`self.K2_CommitAbility`))
  (if _returnvalue_2
    (`self.SetAbilityValues`)
    (`/Engine/EditorBlueprintResources/StandardMacros.IsValid` _attackanimation :!label _label
      (:`Is Valid`
        (set `self.AnimOver` false)
        (if _usesforwardrootmotion
          (`AbilityTask_ApplyRootMotionMoveToForce.ApplyRootMotionMoveToForce` "None" (+ (* (`Actor.GetActorForwardVector` _returnvalue) _rootmotionforce) (`Actor.K2_GetActorLocation` _returnvalue)) _rootmotionduration false "MOVE_None" false null "MaintainLastRootMotionVelocity"
            (:`then`
              _)))
        (`AbilityTask_PlayMontageAndWait.CreatePlayMontageAndWaitProxy` "None" _attackanimation _attackanimplayrate "None" false
          (:`then`
            (set `self.WaitingForInput` true)
            (`KismetSystemLibrary.PrintString` "WARNING: Attack Chain Waiting For Input" true true (struct :`R` 1.0 :`G` 0.549291 :`A` 1.0) 1.0 "MeleeWaitingInput")
            (bind (_asynctaskproxy _payload) (`AbilityTask_WaitGameplayEvent.WaitGameplayEvent` (struct :`TagName` "Tests.Event.Hit") null true)
              (:`then`
                (`AbilityTask_WaitInputRelease.WaitInputRelease` true
                  (:`OnRelease`
                    (set `self.ButtonWasReleased` true)
                    (`self.CustomEndAbility`))))
              (:`EventReceived`
                (bind _gameplayeffectspechandle (`/Game/Libraries/FunctionLibrary.Make Gameplay Effect Damage` (`self.GetAvatarActorFromActorInfo`) (`.AttackDamageMultiplier_17_0BA6DCAF4CAFB2F68D0519B827BF07E2` (break `/Game/GAS/AbilityInfo/MeleeAbilityInfo_Attack` (`|GetArrayItem` (`self.Struct Melee Info Attacks`) (`self.CurrentAttack`))))))
                (bind (_eventtag _instigator _target _optionalobject _optionalobject2 _contexthandle _instigatortags _targettags _eventmagnitude _targetdata) (break `GameplayEventData` _payload))
                (`self.K2_ApplyGameplayEffectSpecToTarget` _gameplayeffectspechandle _targetdata)
                ;[1 1 1] Debug: Print hit target names
                (for _array_element (`AbilitySystemBlueprintLibrary.GetActorsFromTargetData` _targetdata)
                  (`KismetSystemLibrary.PrintString` (`KismetTextLibrary.Conv_TextToString` (`|FormatText` "Target hit: {Target Name}" (`KismetTextLibrary.Conv_StringToText` (`KismetSystemLibrary.GetDisplayName` _array_element)))) true true (struct :`R` 0.806952 :`G` 0.417885 :`A` 1.0) 2.0 "None")))))
          (:`OnCompleted`
            (set `self.AnimOver` false :!label _label_2)
            (`AbilityTask_PlayMontageAndWait.CreatePlayMontageAndWaitProxy` "None" _recoveryanimation _recoveryanimplayrate "None" false
              (:`then`
                (if (not (`self.AutoChain`))
                  (`AbilityTask_WaitInputRelease.WaitInputRelease` true
                    (:`OnRelease`
                      _)))
                (`AbilityTask_WaitInputPress.WaitInputPress` false
                  (:`OnPress`
                    (set `self.ButtonWasReleased` false)
                    (`KismetSystemLibrary.PrintString` "WARNING: Attack Chain Continue: Input Received" true true (struct :`R` 0.05007 :`G` 1.0 :`A` 1.0) 1.0 "MeleeInputReceived")
                    (`/Engine/EditorBlueprintResources/StandardMacros.IncrementInt` (`self.CurrentAttack`)
                      (:`  `
                        (goto _label))))))
              (:`OnCompleted`
                _)
              (:`OnBlendOut`
                _)
              (:`OnInterrupted`
                _)
              (:`OnCancelled`
                _))
            (set `self.AnimOver` true)
            (set `self.WaitingForInput` false)
            (`self.CustomEndAbility`))
          (:`OnBlendOut`
            (goto _label_2))
          (:`OnInterrupted`
            (goto _label_2))
          (:`OnCancelled`
            (goto _label_2))))
      (:`Is Not Valid`
        (`KismetSystemLibrary.PrintText` (`|FormatText` "WARNING: Attack Animation Number {index}: Not Valid" _currentattack))
        (`self.CustomEndAbility` :!label _label_3)))
    (else
      (goto _label_3))))

(event `SetAbilityValues`
  (bind (_struct_meleeinfo_canattackloop _struct_meleeinfo_canattackautochain _struct_meleeinfo_attackchain) (break `/Game/GAS/AbilityInfo/MeleeAbilityInfo` (`/Game/Weapons/BComp_WeaponHandler.Struct_MeleeInfo` (`Actor.GetComponentByClass` (`self.GetAvatarActorFromActorInfo`) "/Game/Weapons/BComp_WeaponHandler.BComp_WeaponHandler_C"))))
  (set `self.Struct Melee Info Attacks` _struct_meleeinfo_attackchain)
  (set `self.Looping` _struct_meleeinfo_canattackloop)
  (set `self.AutoChain` _struct_meleeinfo_canattackautochain))

(event `CustomEndAbility`
  (if (<= (`KismetArrayLibrary.Array_Length` (`self.Struct Melee Info Attacks`)) (`self.CurrentAttack`))
    (if (not (`self.Looping`))
      (`AbilityTask_WaitInputRelease.WaitInputRelease` false
        (:`OnRelease`
          _)))
    (`self.K2_EndAbility` :!label _label_4)
    (elif (and (`self.ButtonWasReleased`) (not (`self.WaitingForInput`)))
      (goto _label_4))))