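; Gameplay ability for a charged ranged shot: holding input charges the weapon, and releasing fires a projectile with damage scaled by hold time.
; Charge limits come from BComp_WeaponHandler; a looping timer draws debug spheres at the muzzle, then auto-fires at full charge if configured.
; Firing builds a damage effect spec, traces from the camera to aim BP_Projectile from the muzzle with clamped rotation, then plays montage, muzzle burst and sound.
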(event `ShowFullyCharged`
  ;[1 1 1] Display Fully Charged Debug Sphere
  (`|ExecutionSequence` :!label _label
    (:`then_0`
      (`KismetSystemLibrary.DrawDebugSphere` (.location (`SceneComponent.GetSocketTransform` (`/Game/Weapons/WeaponBase/B_BaseWeaponInstance.WeaponMesh` (`/Game/Weapons/BComp_WeaponHandler.Weapon Ref` (`Actor.GetComponentByClass` (`self.GetAvatarActorFromActorInfo`) "/Game/Weapons/BComp_WeaponHandler.BComp_WeaponHandler_C"))) "Muzzle" "RTS_World")) 10.0 12 (struct :`R` 1.0 :`B` 0.042986 :`A` 1.0) 0.1 1.0))
    (:`then_1`
      (`KismetSystemLibrary.Delay` 0.1)
      (goto _label))))

(event `self.K2_ActivateAbility`
  (bind _remainingchargeduration (`self.RemainingChargeDuration`))
  (bind _returnvalue (`Actor.GetComponentByClass` (`self.GetAvatarActorFromActorInfo`) "/Game/Weapons/BComp_WeaponHandler.BComp_WeaponHandler_C"))
  (bind _returnvalue_2 (`Actor.GetComponentByClass` (`self.GetAvatarActorFromActorInfo`) "/Script/Engine.CameraComponent"))
  (bind (_returnvalue_roll _returnvalue_pitch _returnvalue_yaw) (`KismetMathLibrary.BreakRotator` (`Actor.K2_GetActorRotation` (`self.GetAvatarActorFromActorInfo`))))
  (bind _returnvalue_3 (/ (`self.FullChargeDuration`) _remainingchargeduration))
  (bind _returnvalue_4 (`SceneComponent.K2_GetComponentLocation` _returnvalue_2))
  (bind _returnvalue_5 (`SceneComponent.GetSocketTransform` (`/Game/Weapons/WeaponBase/B_BaseWeaponInstance.WeaponMesh` (`/Game/Weapons/BComp_WeaponHandler.Weapon Ref` _returnvalue)) "Muzzle" "RTS_World"))
  (bind _location (.location _returnvalue_5))
  (bind _location_2 (.location _returnvalue_5))
  (`self.K2_CommitAbility`)
  (`self.SetAbilityValues`)
  (bind (_asynctaskproxy _timeheld) (`AbilityTask_WaitInputRelease.WaitInputRelease` false)
    (:`then`
      (`AbilityTask_PlayMontageAndWait.CreatePlayMontageAndWaitProxy` "None" "/Game/Characters/Mannequins/Animations/AnimStarterPack/Fire_Rifle_Hip_Montage.Fire_Rifle_Hip_Montage" 0.1
        (:`then`
          ;[1 1 1] Display Updating Charging Debug Sphere
          (if (not (<= (`self.RemainingChargeDuration`) 0.2)) :!label _label_2
            (`KismetSystemLibrary.DrawDebugSphere` (.location (`SceneComponent.GetSocketTransform` (`/Game/Weapons/WeaponBase/B_BaseWeaponInstance.WeaponMesh` (`/Game/Weapons/BComp_WeaponHandler.Weapon Ref` (`Actor.GetComponentByClass` (`self.GetAvatarActorFromActorInfo`) "/Game/Weapons/BComp_WeaponHandler.BComp_WeaponHandler_C"))) "Muzzle" "RTS_World")) (- 20.0 _returnvalue_3) 12 (make `LinearColor` _returnvalue_3 (/ _remainingchargeduration (`self.FullChargeDuration`))) 0.1 1.0)
            (bind _output_get (set `self.RemainingChargeDuration` (- (`self.RemainingChargeDuration`) 0.1)))
            (`KismetSystemLibrary.PrintString` (`KismetStringLibrary.Conv_DoubleToString` _output_get))
            (`KismetSystemLibrary.Delay` 0.1)
            (goto _label_2)
            (elif (`self.ForceShotAtFullCharge`)
              (set `self.DamageMultiplier` (`self.Max`))
              (bind _gameplayeffectspechandle (`/Game/Libraries/FunctionLibrary.Make Gameplay Effect Damage` (`self.GetAvatarActorFromActorInfo`) (`self.DamageMultiplier`) :!label _label_3))
              ;[1 1 1] Line traces from camera to check if aim needs to get adjusted for closer objects
              (bind (_outhit _returnvalue_6) (`KismetSystemLibrary.LineTraceSingleForObjects` :`Start` _returnvalue_4 :`End` (+ _returnvalue_4 (* (`SceneComponent.GetForwardVector` _returnvalue_2) 3000.0)) :`ObjectTypes` (`|MakeArray` "ObjectTypeQuery1" "ObjectTypeQuery3" :!type "EObjectTypeQuery Enum") :`DrawTime` 1.5))
              (bind (_bblockinghit _binitialoverlap _time _distance _location_3 _impactpoint _normal _impactnormal _physmat _hitactor _hitcomponent _hitbonename _bonename _hititem _elementindex _faceindex _tracestart _traceend) (`GameplayStatics.BreakHitResult` _outhit))
              (`|SpawnActorFromClass` "/Game/Weapons/WeaponBase/BP_Projectile.BP_Projectile_C" (`KismetMathLibrary.MakeTransform` _location_2 (`/Game/Libraries/FunctionLibrary.ClampProjectileRotation` _returnvalue_yaw (.roll (`KismetMathLibrary.Conv_VectorToRotator` (`KismetMathLibrary.GetDirectionUnitVector` _location_2 (`KismetMathLibrary.SelectVector` _impactpoint _traceend _returnvalue_6)))) (.pitch (`KismetMathLibrary.Conv_VectorToRotator` (`KismetMathLibrary.GetDirectionUnitVector` _location_2 (`KismetMathLibrary.SelectVector` _impactpoint _traceend _returnvalue_6)))) (.yaw (`KismetMathLibrary.Conv_VectorToRotator` (`KismetMathLibrary.GetDirectionUnitVector` _location_2 (`KismetMathLibrary.SelectVector` _impactpoint _traceend _returnvalue_6)))) (`.ProjectileRotationClamp_15_3932B28F4C5FA4F5218A4FBEDA5A4717` (break `/Game/GAS/AbilityInfo/RangedAbilityInfo` (`/Game/Weapons/BComp_WeaponHandler.Struct_RangedInfo` _returnvalue))))) "Undefined" "MultiplyWithRoot" (`self.GetAvatarActorFromActorInfo`) _gameplayeffectspechandle null)
              (`AbilityTask_PlayMontageAndWait.CreatePlayMontageAndWaitProxy` "None" "/Game/Characters/Mannequins/Animations/AnimStarterPack/Fire_Rifle_Ironsights_Montage.Fire_Rifle_Ironsights_Montage"
                (:`then`
                  (`NiagaraFunctionLibrary.SpawnSystemAtLocation` "/Game/VFX/NS_MuzzleBurst.NS_MuzzleBurst" _location (.rotation _returnvalue_5))
                  (`GameplayStatics.PlaySoundAtLocation` "/Game/SFX/SC_GunShot_01.SC_GunShot_01" _location (struct) 0.4 1.5 0.0 null null null null)
                  (`AbilityTask_WaitInputRelease.WaitInputRelease` true
                    (:`OnRelease`
                      (`self.K2_EndAbility`)))))
              (else
                (`self.ShowFullyCharged`)))))))
    (:`OnRelease`
      (set `self.DamageMultiplier` (`KismetMathLibrary.Lerp` (`self.Min`) (`self.Max`) (/ _timeheld (`self.FullChargeDuration`))))
      (goto _label_3))))

(event `SetAbilityValues`
  (bind (_struct_rangedinfo_projectilerotationclamp _struct_rangedinfo_forceshotatfullcharge _struct_rangedinfo_fullchargeduration _struct_rangedinfo_mindamagemultiplier _struct_rangedinfo_maxdamagemultiplier) (break `/Game/GAS/AbilityInfo/RangedAbilityInfo` (`/Game/Weapons/BComp_WeaponHandler.Struct_RangedInfo` (`Actor.GetComponentByClass` (`self.GetAvatarActorFromActorInfo`) "/Game/Weapons/BComp_WeaponHandler.BComp_WeaponHandler_C"))))
  ;[1 1 1] Get Ability Values from weapon handler
  (set `self.ForceShotAtFullCharge` _struct_rangedinfo_forceshotatfullcharge)
  (set `self.Min` _struct_rangedinfo_mindamagemultiplier)
  (set `self.Max` _struct_rangedinfo_maxdamagemultiplier)
  (set `self.FullChargeDuration` _struct_rangedinfo_fullchargeduration)
  (set `self.RemainingChargeDuration` (`self.FullChargeDuration`)))