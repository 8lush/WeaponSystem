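; Gameplay ability for instant melee attacks that plays the attack montage chain read from the avatar's weapon handler component.
; Each swing can add a short forward root-motion force, and a hit gameplay event applies a damage effect scaled by that attack's multiplier.
; Holding input advances through the chain, while releasing it lets the current swing finish before the ability ends.
; The looping flag only affects how the chain's end is handled.
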(event `self.K2_OnEndAbility`
  (params (bWasCancelled :type Boolean))
  (`KismetSystemLibrary.PrintString` "Ability Ended" true true (struct :`G` 0.66 :`B` 1.0 :`A` 1.0) 2.0 "AbilityEnded"))

(event `self.K2_ActivateAbility`
  (bind _returnvalue (`self.GetAvatarActorFromActorInfo`))
  (bind _currentattack (`self.CurrentAttack`))
  (bind (_attackanimation _animplayrate) (break `/Game/GAS/AbilityInfo/MeleeAbilityInfo_Attack` (`|GetArrayItem` (`self.Struct Melee Info Attacks`) _currentattack)))
  (bind _returnvalue_2 (`self.K2_CommitAbility`))
  (if _returnvalue_2
    (`self.SetAbilityValues`)
    (`/Engine/EditorBlueprintResources/StandardMacros.IsValid` _attackanimation :!label _label
      (:`Is Valid`
        (set `self.AnimOver` false)
        (if (`self.RootMotion`)
          (`AbilityTask_ApplyRootMotionMoveToForce.ApplyRootMotionMoveToForce` "None" (+ (* (`Actor.GetActorForwardVector` _returnvalue) 50.0) (`Actor.K2_GetActorLocation` _returnvalue)) 0.2 false "MOVE_None" false null "MaintainLastRootMotionVelocity"
            (:`then`
              _)))
        (`AbilityTask_PlayMontageAndWait.CreatePlayMontageAndWaitProxy` "None" _attackanimation _animplayrate
          (:`then`
            (bind (_asynctaskproxy _payload) (`AbilityTask_WaitGameplayEvent.WaitGameplayEvent` (struct :`TagName` "Tests.Event.Hit") null true)
              (:`then`
                (`AbilityTask_WaitInputRelease.WaitInputRelease` false
                  (:`OnRelease`
                    (if (`self.AnimOver`)
                      (`self.K2_EndAbility`)
                      (else
                        (set `self.InputReleased` true))))))
              (:`EventReceived`
                (bind _gameplayeffectspechandle (`/Game/Libraries/FunctionLibrary.Make Gameplay Effect Damage` (`self.GetAvatarActorFromActorInfo`) (`.DamageMultiplier_9_0BA6DCAF4CAFB2F68D0519B827BF07E2` (break `/Game/GAS/AbilityInfo/MeleeAbilityInfo_Attack` (`|GetArrayItem` (`self.Struct Melee Info Attacks`) (`self.CurrentAttack`))))))
                (bind (_eventtag _instigator _target _optionalobject _optionalobject2 _contexthandle _instigatortags _targettags _eventmagnitude _targetdata) (break `GameplayEventData` _payload))
                (`self.K2_ApplyGameplayEffectSpecToTarget` _gameplayeffectspechandle _targetdata)
                ;[1 1 1] Debug: Print hit target names
                (for _array_element (`AbilitySystemBlueprintLibrary.GetActorsFromTargetData` _targetdata)
                  (`KismetSystemLibrary.PrintString` (`KismetTextLibrary.Conv_TextToString` (`|FormatText` "Target hit: {Target Name}" (`KismetTextLibrary.Conv_StringToText` (`KismetSystemLibrary.GetDisplayName` _array_element)))) true true (struct :`R` 0.806952 :`G` 0.417885 :`A` 1.0) 2.0 "None")))))
          (:`OnCompleted`
            (set `self.AnimOver` true :!label _label_2)
            (`/Engine/EditorBlueprintResources/StandardMacros.IncrementInt` (`self.CurrentAttack`)
              (:`  `
                (if (<= (`KismetArrayLibrary.Array_Length` (`self.Struct Melee Info Attacks`)) (`self.CurrentAttack`))
                  (if (not (`self.Looping`))
                    (if (`self.InputReleased`)
                      (`self.K2_EndAbility` :!label _label_3))
                    (else
                      (goto _label_3)))
                  (elif (`self.InputReleased`)
                    (goto _label_3)
                    (else
                      (goto _label)))))))
          (:`OnBlendOut`
            (goto _label_2))
          (:`OnInterrupted`
            (goto _label_2))
          (:`OnCancelled`
            (goto _label_2))))
      (:`Is Not Valid`
        (`KismetSystemLibrary.PrintText` (`|FormatText` "WARNING: Attack Animation Number {index}: Not Valid" _currentattack))
        (goto _label_3)))
    (else
      (goto _label_3))))

(event `SetAbilityValues`
  (bind (_struct_meleeinfo_canattackloop _struct_meleeinfo_usesrootmotion _struct_meleeinfo_attackchain) (break `/Game/GAS/AbilityInfo/MeleeAbilityInfo` (`/Game/Weapons/BComp_WeaponHandler.Struct_MeleeInfo` (`Actor.GetComponentByClass` (`self.GetAvatarActorFromActorInfo`) "/Game/Weapons/BComp_WeaponHandler.BComp_WeaponHandler_C"))))
  (set `self.Struct Melee Info Attacks` _struct_meleeinfo_attackchain)
  (set `self.Looping` _struct_meleeinfo_canattackloop)
  (set `self.RootMotion` _struct_meleeinfo_usesrootmotion))