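; Deprecated first-version gameplay ability for a melee punch that hits every valid target in a radius ahead of the owner.
; After committing, it starts a tiny forward root-motion jump and a sped-up punch montage, then immediately runs instant radius targeting with debug enabled.
; It applies GE_BasicDamage to hit actors with an ability system component, excluding itself, and prints debug messages.
; The ability ends when the montage finishes or the commit fails.
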(event `self.K2_ActivateAbility`
  (bind _returnvalue (`self.GetOwningActorFromActorInfo`))
  (bind _returnvalue_2 (`self.K2_CommitAbility`))
  (if _returnvalue_2
    (`AbilityTask_ApplyRootMotionJumpForce.ApplyRootMotionJumpForce` "None" (`KismetMathLibrary.Conv_VectorToRotator` (`Actor.GetActorForwardVector` (`self.GetAvatarActorFromActorInfo`))) 5.0 0.0 0.02 0.0 true "SetVelocity"
      (:`then`
        (`AbilityTask_PlayMontageAndWait.CreatePlayMontageAndWaitProxy` "None" "/Game/Ninja_Starter/Animation/IPC/AM_TestPunch.AM_TestPunch" 2.0
          (:`then`
            (bind (_asynctaskproxy _data) (`AbilityTask_WaitTargetData.WaitTargetData` "None" "Instant" "/Script/GameplayAbilities.GameplayAbilityTargetActor_Radius" 200.0 (make `GameplayAbilityTargetingLocationInfo` "LiteralTransform" (`KismetMathLibrary.Conv_VectorToTransform` (+ (`Actor.K2_GetActorLocation` _returnvalue) (* (`Actor.GetActorForwardVector` _returnvalue) 100.0)))) (struct) "/Script/GameplayAbilities.GameplayAbilityWorldReticle" (struct) true)
              (:`ValidData`
                ;[1 1 1] Loop through all targets hit
                (for _array_element (`AbilitySystemBlueprintLibrary.GetAllActorsFromTargetData` _data)
                  (bind _returnvalue_3 (`AbilitySystemBlueprintLibrary.GetAbilitySystemComponent` _array_element))
                  ;[1 1 1] Check if target has a GAS component
                  (`/Engine/EditorBlueprintResources/StandardMacros.IsValid` _returnvalue_3
                    (:`Is Valid`
                      ;[1 1 1] Ignore Self
                      (if (!= _returnvalue_3 (`self.GetAbilitySystemComponentFromActorInfo`))
                        (`self.BP_ApplyGameplayEffectToTarget` (`AbilitySystemBlueprintLibrary.AbilityTargetDataFromActor` _array_element) "/Game/GAS/GameplayEffects/GE_BasicDamage.GE_BasicDamage_C")
                        (`KismetSystemLibrary.PrintString` "TargetHit"))))))))
          (:`OnCompleted`
            (`self.K2_EndAbility` :!label _label))
          (:`OnBlendOut`
            (goto _label))
          (:`OnInterrupted`
            (goto _label))
          (:`OnCancelled`
            (goto _label)))))
    (else
      (goto _label))))

(event `self.K2_OnEndAbility`
  (params (bWasCancelled :type Boolean))
  (`KismetSystemLibrary.PrintString` "Ability Ended" true true (struct :`G` 0.66 :`B` 1.0 :`A` 1.0) 2.0 "AbilityEnded"))