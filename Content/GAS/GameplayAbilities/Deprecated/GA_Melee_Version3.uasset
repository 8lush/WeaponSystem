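; GA_Melee_Version3 is a deprecated melee Gameplay Ability that plays chained attack montages from an array while input stays held.
; On activation it commits, optionally lunges the avatar forward with root-motion MoveToForce, then starts the current montage.
; A one-shot hit gameplay event applies a damage effect to its target data and prints target names.
; Montage end advances the chain index, while input-release tracking decides when the ability ends.
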(event `self.K2_ActivateAbility`
  (bind _returnvalue (`self.GetAvatarActorFromActorInfo`))
  (bind _currentattack (`self.CurrentAttack`))
  (bind _output (`|GetArrayItem` (`self.AttackChainMontages`) _currentattack))
  (bind _returnvalue_2 (`self.K2_CommitAbility`))
  (if _returnvalue_2
    (if (`self.RootMotion`)
      (`AbilityTask_ApplyRootMotionMoveToForce.ApplyRootMotionMoveToForce` "None" (+ (* (`Actor.GetActorForwardVector` _returnvalue) 50.0) (`Actor.K2_GetActorLocation` _returnvalue)) 0.2 false "MOVE_None" false null "MaintainLastRootMotionVelocity"
        (:`then`
          (`/Engine/EditorBlueprintResources/StandardMacros.IsValid` _output :!label _label
            (:`Is Valid`
              (`AbilityTask_PlayMontageAndWait.CreatePlayMontageAndWaitProxy` "None" _output (`self.AnimPlayRate`) :!label _label_2
                (:`then`
                  (bind (_asynctaskproxy _payload) (`AbilityTask_WaitGameplayEvent.WaitGameplayEvent` (struct :`TagName` "Tests.Event.Hit") null true)
                    (:`then`
                      (`AbilityTask_WaitInputRelease.WaitInputRelease` false
                        (:`OnRelease`
                          (if (`self.AnimOver`)
                            (`self.K2_EndAbility`)
                            (else
                              (set `self.InputReleased` true))))))
                    (:`EventReceived`
                      (bind _gameplayeffectspechandle (`/Game/Libraries/FunctionLibrary.Make Gameplay Effect Damage` (`self.GetAvatarActorFromActorInfo`)))
                      (bind (_eventtag _instigator _target _optionalobject _optionalobject2 _contexthandle _instigatortags _targettags _eventmagnitude _targetdata) (break `GameplayEventData` _payload))
                      (`self.K2_ApplyGameplayEffectSpecToTarget` _gameplayeffectspechandle _targetdata)
                      ;[1 1 1] Debug: Print hit target names
                      (for _array_element (`AbilitySystemBlueprintLibrary.GetActorsFromTargetData` _targetdata)
                        (`KismetSystemLibrary.PrintString` (`KismetTextLibrary.Conv_TextToString` (`|FormatText` "Target hit: {Target Name}" (`KismetTextLibrary.Conv_StringToText` (`KismetSystemLibrary.GetDisplayName` _array_element)))) true true (struct :`R` 0.806952 :`G` 0.417885 :`A` 1.0) 2.0 "None")))))
                (:`OnCompleted`
                  (set `self.AnimOver` true :!label _label_3)
                  (`/Engine/EditorBlueprintResources/StandardMacros.IncrementInt` (`self.CurrentAttack`)
                    (:`  `
                      (if (<= (`KismetArrayLibrary.Array_Length` (`self.AttackChainMontages`)) (`self.CurrentAttack`))
                        (if (not (`self.Looping`))
                          (if (`self.InputReleased`)
                            (`self.K2_EndAbility` :!label _label_4))
                          (else
                            (goto _label_4)))
                        (elif (`self.InputReleased`)
                          (goto _label_4)
                          (else
                            (goto _label)))))))
                (:`OnBlendOut`
                  (goto _label_3))
                (:`OnInterrupted`
                  (goto _label_3))
                (:`OnCancelled`
                  (goto _label_3))))
            (:`Is Not Valid`
              (`KismetSystemLibrary.PrintText` (`|FormatText` "WARNING: Attack Animation Number {index}: Not Valid" _currentattack))
              (goto _label_4)))))
      (else
        (goto _label_2)))
    (else
      (goto _label_4))))

(event `self.K2_OnEndAbility`
  (params (bWasCancelled :type Boolean))
  (`KismetSystemLibrary.PrintString` "Ability Ended" true true (struct :`G` 0.66 :`B` 1.0 :`A` 1.0) 2.0 "AbilityEnded"))