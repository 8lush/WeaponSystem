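; Gameplay ability for a melee punch that damages actors within a radius in front of the owner.
; On commit, it applies a tiny forward root-motion jump and plays the punch montage, ending when the montage finishes or stops.
; As the montage starts, an instant radius target-data check at Range gathers actors, with an optional debug sphere.
; Each hit actor with a different ability system component receives the configured GameplayEffect with SetByCaller damage.
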(event `self.K2_ActivateAbility`
  (bind _returnvalue (`self.GetOwningActorFromActorInfo`))
  (bind _returnvalue_2 (+ (`Actor.K2_GetActorLocation` _returnvalue) (* (`Actor.GetActorForwardVector` _returnvalue) (`self.Range`))))
  (bind _returnvalue_3 (`self.K2_CommitAbility`))
  (if _returnvalue_3
    (`AbilityTask_ApplyRootMotionJumpForce.ApplyRootMotionJumpForce` "None" (`KismetMathLibrary.Conv_VectorToRotator` (`Actor.GetActorForwardVector` (`self.GetAvatarActorFromActorInfo`))) 5.0 0.0 0.02 0.0 true "SetVelocity"
      (:`then`
        (`AbilityTask_PlayMontageAndWait.CreatePlayMontageAndWaitProxy` "None" "/Game/Ninja_Starter/Animation/IPC/AM_TestPunch.AM_TestPunch" 2.0
          (:`then`
            (bind (_asynctaskproxy _data) (`AbilityTask_WaitTargetData.WaitTargetData` "None" "Instant" "/Script/GameplayAbilities.GameplayAbilityTargetActor_Radius" (`self.Radius`) (make `GameplayAbilityTargetingLocationInfo` "LiteralTransform" (`KismetMathLibrary.Conv_VectorToTransform` _returnvalue_2)) (struct) null)
              (:`then`
                (if (`self.IsDebug?`)
                  (`KismetSystemLibrary.DrawDebugSphere` _returnvalue_2 (`self.Radius`) 12 (struct :`R` 0.614583 :`B` 0.011736 :`A` 1.0) 1.0)))
              (:`ValidData`
                ;[1 1 1] Loop through all targets hit
                (for _array_element (`AbilitySystemBlueprintLibrary.GetAllActorsFromTargetData` _data)
                  (bind _returnvalue_4 (`AbilitySystemBlueprintLibrary.GetAbilitySystemComponent` _array_element))
                  ;[1 1 1] Check if target has a GAS component
                  (`/Engine/EditorBlueprintResources/StandardMacros.IsValid` _returnvalue_4
                    (:`Is Valid`
                      ;[1 1 1] Ignore Self
                      (if (!= _returnvalue_4 (`self.GetAbilitySystemComponentFromActorInfo`))
                        (bind _returnvalue_5 (`AbilitySystemBlueprintLibrary.AssignTagSetByCallerMagnitude` (`self.MakeOutgoingGameplayEffectSpec` (`self.GameplayEffect`)) (struct :`TagName` "Damage.SetByCaller") (`self.Damage`)))
                        (`self.K2_ApplyGameplayEffectSpecToTarget` _returnvalue_5 (`AbilitySystemBlueprintLibrary.AbilityTargetDataFromActor` _array_element))
                        (`KismetSystemLibrary.PrintString` "TargetHit"))))))))
          (:`OnCompleted`
            (`self.K2_EndAbility` :!label _label))
          (:`OnBlendOut`
            (goto _label))
          (:`OnInterrupted`
            (goto _label))
          (:`OnCancelled`
            (goto _label)))))
    (else
      (goto _label))))

(event `self.K2_OnEndAbility`
  (params (bWasCancelled :type Boolean))
  (`KismetSystemLibrary.PrintString` "Ability Ended" true true (struct :`G` 0.66 :`B` 1.0 :`A` 1.0) 2.0 "AbilityEnded"))