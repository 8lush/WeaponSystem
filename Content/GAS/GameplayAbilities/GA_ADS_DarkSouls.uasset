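; Gameplay ability for aim-down-sights on the Dark Souls-style character, held for as long as the input is pressed.
; On activation it commits, starts aim and camera zoom through the avatar's BComp_WeaponHandler component, and switches the character's HUD to aim state.
; An input-release wait ends the ability, and its end event reverses the aim, zoom and HUD changes.
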(event `self.K2_ActivateAbility`
  (bind _returnvalue (`self.GetAvatarActorFromActorInfo`))
  (bind _returnvalue_2 (`Actor.GetComponentByClass` _returnvalue "/Game/Weapons/BComp_WeaponHandler.BComp_WeaponHandler_C"))
  (`self.K2_CommitAbility`)
  (`/Game/Weapons/BComp_WeaponHandler.AimStart` _returnvalue_2)
  (`/Game/Weapons/BComp_WeaponHandler.ZoomCamera` _returnvalue_2)
  (bind _asbp_dark_souls_character (cast `/Game/Prototypes/PrototypeAssets/BP_DarkSoulsCharacter` _returnvalue))
  (`/Game/UI/WB_PlayerHUD_DarkSouls.AIM` (`/Game/Prototypes/PrototypeAssets/BP_DarkSoulsCharacter.HUD` _asbp_dark_souls_character))
  (`AbilityTask_WaitInputRelease.WaitInputRelease` false
    (:`OnRelease`
      (`self.K2_EndAbility`))))

(event `self.K2_OnEndAbility`
  (params (bWasCancelled :type Boolean))
  (bind _returnvalue (`self.GetAvatarActorFromActorInfo`))
  (`/Game/Weapons/BComp_WeaponHandler.AimEnd` (`Actor.GetComponentByClass` (`self.GetAvatarActorFromActorInfo`) "/Game/Weapons/BComp_WeaponHandler.BComp_WeaponHandler_C"))
  (`/Game/Weapons/BComp_WeaponHandler.EndZoomCamera` (`Actor.GetComponentByClass` _returnvalue "/Game/Weapons/BComp_WeaponHandler.BComp_WeaponHandler_C"))
  (bind _asbp_dark_souls_character (cast `/Game/Prototypes/PrototypeAssets/BP_DarkSoulsCharacter` _returnvalue))
  (`/Game/UI/WB_PlayerHUD_DarkSouls.ENDAIM` (`/Game/Prototypes/PrototypeAssets/BP_DarkSoulsCharacter.HUD` _asbp_dark_souls_character)))