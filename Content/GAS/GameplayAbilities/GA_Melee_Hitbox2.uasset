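; Gameplay Ability for a melee attack that damages each target hit during its montage once.
; On commit, it nudges the avatar forward with root motion MoveToForce, plays the montage and listens for Tests.Event.Hit events.
; New targets are recorded in TargetsHit and receive a GameplayEffect with SetByCaller damage from the event's TargetData.
; It ends on montage exit or failed commit, printing debug messages for hits and ending.
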(event `self.K2_ActivateAbility`
  (bind _returnvalue (`self.GetAvatarActorFromActorInfo`))
  (bind _returnvalue_2 (`self.K2_CommitAbility`))
  (if _returnvalue_2
    (`AbilityTask_ApplyRootMotionMoveToForce.ApplyRootMotionMoveToForce` "None" (+ (* (`Actor.GetActorForwardVector` _returnvalue) 50.0) (`Actor.K2_GetActorLocation` _returnvalue)) 0.2 false "MOVE_None" false null "MaintainLastRootMotionVelocity"
      (:`then`
        (`AbilityTask_PlayMontageAndWait.CreatePlayMontageAndWaitProxy` "None" (`self.Montage to Play`) (`self.AnimPlayRate`)
          (:`then`
            (bind (_asynctaskproxy _payload) (`AbilityTask_WaitGameplayEvent.WaitGameplayEvent` (struct :`TagName` "Tests.Event.Hit") null)
              (:`EventReceived`
                (bind (_eventtag _instigator _target _optionalobject _optionalobject2 _contexthandle _instigatortags _targettags _eventmagnitude _targetdata) (break `GameplayEventData` _payload))
                ;[1 1 1] Make Array of Hit Targets (to avoid hitting same target twice)
                (if (not (`KismetArrayLibrary.Array_Contains` (`self.TargetsHit`) _target))
                  (`KismetArrayLibrary.Array_Add` (`self.TargetsHit`) _target)
                  ;[1 1 1] Make GameplaySpec and Apply GameplayEffect
                  (bind _returnvalue_3 (`AbilitySystemBlueprintLibrary.AssignTagSetByCallerMagnitude` (`self.MakeOutgoingGameplayEffectSpec` (`self.GameplayEffect`)) (struct :`TagName` "Damage.SetByCaller") (`self.Damage`)))
                  (`self.K2_ApplyGameplayEffectSpecToTarget` _returnvalue_3 _targetdata)
                  ;[1 1 1] Debug - Print Targets Hit
                  (for _array_element (`AbilitySystemBlueprintLibrary.GetActorsFromTargetData` _targetdata)
                    (`KismetSystemLibrary.PrintString` (`KismetTextLibrary.Conv_TextToString` (`|FormatText` "Target hit: {Target Name}" (`KismetTextLibrary.Conv_StringToText` (`KismetSystemLibrary.GetDisplayName` _array_element)))) true true (struct :`R` 0.806952 :`G` 0.417885 :`A` 1.0) 2.0 "TargetHit"))))))
          (:`OnCompleted`
            (`self.K2_EndAbility` :!label _label))
          (:`OnBlendOut`
            (goto _label))
          (:`OnInterrupted`
            (goto _label))
          (:`OnCancelled`
            (goto _label)))))
    (else
      (goto _label))))

(event `self.K2_OnEndAbility`
  (params (bWasCancelled :type Boolean))
  ;[1 1 1] Debug - print when ability has ended
  (`KismetSystemLibrary.PrintText` (`|FormatText` "WARNING: {Ability} Ended!" (`KismetSystemLibrary.GetDisplayName` self)) true true (struct :`R` 0.564872 :`G` 0.17844 :`B` 0.744792 :`A` 1.0)))