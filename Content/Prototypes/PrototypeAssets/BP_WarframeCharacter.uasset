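; Prototype Warframe character Blueprint that puts the player HUD on screen at play start.
; BeginPlay creates a WB_PlayerHUD widget and adds it to the player screen.
; A debug event loops every second, printing the character's name and an Ability System attribute, apparently health, under a per-character key, but its only call is disconnected, so it never runs.
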(event `DebugPrintPlayerHealth`
  (bind _returnvalue (`KismetSystemLibrary.GetDisplayName` self))
  ;[1 1 1] Debug Print Player Health
  (`|ExecutionSequence` :!label _label
    (:`then_0`
      (`KismetSystemLibrary.PrintString` (`KismetStringLibrary.Concat_StrStr` _returnvalue ": " (`KismetStringLibrary.Conv_DoubleToString` (`.ReturnValue` (`AbilitySystemComponent.GetGameplayAttributeValue` (`self.AbilitySystemComponent`) (struct :`AttributeName` "Health" :`Attribute` "/Script/WeaponSystem.BasicCharacterAttributeSet:Health" :`AttributeOwner` "/Script/CoreUObject.Class'\"/Script/WeaponSystem.BasicCharacterAttributeSet\"'"))))) true false (struct :`G` 1.0 :`B` 0.104963 :`A` 1.0) 2.0 (`KismetStringLibrary.Conv_StringToName` _returnvalue)))
    (:`then_1`
      (`KismetSystemLibrary.Delay` 1.0)
      (goto _label))))

(event `self.ReceiveBeginPlay`
  (bind _returnvalue (`|CreateWidget` "/Game/UI/WB_PlayerHUD.WB_PlayerHUD_C"))
  (`UserWidget.AddToPlayerScreen` _returnvalue 0))

(fn `UserConstructionScript`)